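; Player controller for a Pixel Streaming viewer that rotates tagged ROTATOR and World actors, opens doors and swaps streamed levels.
; Mouse, wheel and menu events drive yaw and sync the W_Menu slider, while doors play a Level Sequence forward or reversed.
; Most changes re-render Bp_Target scene captures in repeated delayed passes.
; Level swaps reset rotation, camera and menu; streaming input is only printed.
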(event Custom|New_Connection_Started
  (params (StreamerId :type String) (PlayerId :type String) (QualityController :type Boolean))
  ;[0 0 0] Bind On New Connection started event (could use this event to do something when a new stream connections is started)
  (Class|PixelStreamingInput|SendPixelStreamingResponse (Variables|Default|GetPixelStreamingInput) "{ \"new_user_connected\": \"true\" }")
  (Development|PrintString "{ \"new_user_connected\": \"true\" }" true true "(R=0.000000,G=0.660000,B=1.000000,A=1.000000)" 2e+01)
  ;[0 0 0] Allows Pixel streaming reponse messages to be sent
  (Variables|Default|SetbAppIsStreaming true))

(event Custom|GET%20ROTATOR
  ;[0 0 0] GET ROTATORS
  (Utilities|FlowControl|Sequence
    (:then_0
      (bind _outactors (Actor|GetAllActorsOfClass "/Script/Engine.Actor"))
      (for _array_element _outactors
        (if (Actor|ActorHasTag _array_element "ROTATOR")
          (Variables|Default|SetROTATOR _array_element))))
    (:then_1
      (bind _outactors_2 (Actor|GetAllActorsOfClass "/Script/Engine.Actor"))
      (for _array_element_2 _outactors_2
        (if (Actor|ActorHasTag _array_element_2 "World")
          (Variables|Default|SetWorld _array_element_2))))))

(event Custom|SliderRot
  (params (rot :type Float%20%28single-precision%29))
  (bind _world (Variables|Default|GetWorld))
  (bind _rotator (Variables|Default|GetROTATOR))
  (bind _returnvalue (Transformation|GetActorRotation _world))
  (bind _returnvalue_2 (Transformation|GetActorRotation _rotator))
  ;[0 0 0] SLIDER ROTATOR
  (Transformation|SetActorRotation _rotator (Math|Rotator|MakeRotator (.roll _returnvalue_2) (.pitch _returnvalue_2) rot))
  (Transformation|SetActorRotation _world (Math|Rotator|MakeRotator (.roll _returnvalue) (.pitch _returnvalue) rot)))

(event Custom|simple%20capture%20views
  ;[0 0 0] CAPTURE SIMPLE VIEWS
  (bind _outactors (Actor|GetAllActorsOfClass "/Game/Blueprint/Bp_Target.Bp_Target_C"))
  (if (> (Variables|Default|Getint) 4) :!label _label
    (Variables|Default|Setint 0)
    (else
      (for _array_element _outactors
        (Utilities|IsValid (Variables|/Game/Blueprint/Bp_Target.Bp_Target_C|GetSceneCaptureComponent2D _array_element)
          (:Is%20Valid
            (Rendering|SceneCapture|CaptureScene (Variables|/Game/Blueprint/Bp_Target.Bp_Target_C|GetSceneCaptureComponent2D _array_element) :!class /Script/Engine.SceneCaptureComponent2D))))
      (Utilities|FlowControl|Delay 0.3)
      (Math|Integer|IncrementInt (Variables|Default|Getint)
        (:%20%20
          (goto _label))))))

(event Custom|AddRotatiocab
  (params (Add :type Boolean))
  (bind _returnvalue (Math|Float|SelectFloat 1e+01 -1e+01 Add))
  (bind _rotator (Variables|Default|GetROTATOR))
  (bind _world (Variables|Default|GetWorld))
  (bind _returnvalue_2 (Transformation|GetActorRotation _rotator))
  (bind _returnvalue_3 (Transformation|GetActorRotation _world))
  (bind _returnvalue_4 (+ (.yaw _returnvalue_3) _returnvalue))
  ;[0 0 0] ROTATOR - BUTTONS
  (Transformation|SetActorRotation _rotator (Math|Rotator|MakeRotator (.roll _returnvalue_2) (.pitch _returnvalue_2) (+ (.yaw _returnvalue_2) _returnvalue)))
  (Transformation|SetActorRotation _world (Math|Rotator|MakeRotator (.roll _returnvalue_3) (.pitch _returnvalue_3) _returnvalue_4))
  (CallFunction|SimpleCaptureViews)
  (Default|UpdateSliderW (Variables|Default|GetW_Menu) _returnvalue_4))

(event Custom|CreateWidgets
  (Utilities|FlowControl|Sequence
    (:then_0
      (bind _returnvalue (UserInterface|CreateWidget "/Game/UI/W_Menu.W_Menu_C"))
      (Variables|Default|SetW_Menu _returnvalue))
    (:then_1
      (UserInterface|Viewport|AddtoViewport (Variables|Default|GetW_Menu) 0))))

(event Custom|Random_Level
  (bind _levels (Variables|Default|GetLevels))
  ;[0 0 0] RANDON LEVEL
  (for _array_element _levels
    (Class|GameplayStatics|UnloadStreamLevelbySoftObjectPtr _array_element true))
  (CallFunction|VisibilityifContains (.OutItem (Utilities|Array|Random _levels))))

(event Custom|FadeStart
  (bind _returnvalue (Game|GetPlayerCameraManager 0))
  (Class|PlayerCameraManager|SetManualCameraFade :self _returnvalue :InFadeAmount 1.0)
  (Utilities|FlowControl|Delay 2.0)
  (CameraFades|StartCameraFade :self _returnvalue :FromAlpha 1.0 :Duration 1.0 :bHoldWhenFinished true))

(event Custom|Visibility%20If%20Contains
  (params (Level :type World%20Soft%20Object%20Reference))
  ;[0 0 0] CHANGE LEVEL
  (if (not (Variables|Default|GetbIsPlay))
    (if (Variables|Default|Getdoor%20open)
      (CallFunction|DoorsClose)
      (Utilities|FlowControl|Delay 1.5))
    (CallFunction|Rot0Force)
    (Default|BlendCamera (Variables|Default|GetAs%20Bp%20Pawn) 3 "NewEnumerator0" false)
    (Variables|/Script/UMG.WidgetSwitcher|SetActiveWidgetIndex (Variables|/Game/UI/W_Menu.W_Menu_C|GetWidgetSwitcher_Materials (Variables|Default|GetW_Menu)) 0)
    (Variables|Default|SetLevel-new Level)
    (if (Utilities|IsValidSoftObjectReference (Variables|Default|GetLevel-old))
      (Class|GameplayStatics|UnloadStreamLevelbySoftObjectPtr (Variables|Default|GetLevel-old) false))
    (Class|GameplayStatics|LoadStreamLevelbySoftObjectPtr Level true false)
    (CallFunction|GETROTATOR)
    (Variables|Default|SetLevel-old (Variables|Default|GetLevel-new))
    (bind _returnvalue (Actor|GetActorOfClass "/Game/Blueprint/Bp_MaterialSwitch01.Bp_MaterialSwitch01_C"))
    (Default|CollectActors _returnvalue)
    (CallFunction|SimpleCaptureViews)
    (Default|UpdateWidgetLight (Variables|Default|GetW_Menu))
    (Default|UpdateSliderW (Variables|Default|GetW_Menu) 0.0)))

(event Custom|Reset_Level_When_Connections_Closed_Event
  (params (StreamerId :type String))
  ;[0 0 0] Bind On All Connections Closed event (could use this event to do something when all stream connections are lost)
  (Development|PrintString "CONNECTION LOST" true true "(R=0.000000,G=0.660000,B=1.000000,A=1.000000)" 2e+01))

(event Custom|FadeEnd
  (bind _returnvalue (Game|GetPlayerCameraManager 0))
  (Class|PlayerCameraManager|SetManualCameraFade :self _returnvalue)
  (Utilities|FlowControl|Delay 2.0)
  (CameraFades|StartCameraFade :self _returnvalue :ToAlpha 1.0 :Duration 1.0 :bHoldWhenFinished true))

(event Custom|Input_Recieved_Event
  (params (Descriptor :type String))
  ;[0 0 0] Input recieved from frontend
  (bind _output_get (Variables|Default|SetDescriptor Descriptor))
  ;[0 0 0] Print the incomming Json Descriptor string as a message to the screen and to the Log
  (Development|PrintString (Utilities|String|Append "----- DESCRIPTOR: " _output_get " -----") true true "(R=0.000000,G=0.660000,B=1.000000,A=1.000000)" 2e+01)
  (switch string ""))

(event Custom|Rotation0
  (bind _rotator (Variables|Default|GetROTATOR))
  (bind _world (Variables|Default|GetWorld))
  (bind _returnvalue (Transformation|GetActorRotation _world))
  (bind _returnvalue_2 (Transformation|GetActorRotation _rotator))
  ;[0 0 0] ROTATE TO 0
  (Utilities|FlowControl|Sequence
    (:then_0
      (Variables|Default|Setrotation (.yaw _returnvalue_2))
      (bind _newtrack_0 (Timeline|Timeline PlayFromStart)
        (:Update
          (Transformation|SetActorRotation _rotator (Math|Rotator|MakeRotator (.roll _returnvalue_2) (.pitch _returnvalue_2) (Math|Float|Lerp (Variables|Default|Getrotation) 0.0 _newtrack_0)))
          (Default|UpdateSliderW (Variables|Default|GetW_Menu) (Math|Float|Lerp (Variables|Default|Getrotation) 0.0 _newtrack_0)))))
    (:then_1
      (Variables|Default|Setrotation_0 (.yaw _returnvalue))
      (bind _newtrack_0_2 (Timeline|Timeline_0 PlayFromStart)
        (:Update
          (Transformation|SetActorRotation _world (Math|Rotator|MakeRotator (.roll _returnvalue) (.pitch _returnvalue) (Math|Float|Lerp (Variables|Default|Getrotation_0) 0.0 _newtrack_0_2))))
        (:Finished
          (CallFunction|SimpleCaptureViews))))))

(event Custom|Fade_IN
  (bind _returnvalue (Game|GetPlayerCameraManager 0))
  (bind _fade_time (Variables|Default|GetFade%20time))
  ;[0 0 0] FADE
  (Class|PlayerCameraManager|SetManualCameraFade :self _returnvalue :InFadeAmount 1.0 :bInFadeAudio true)
  (Utilities|FlowControl|Delay _fade_time)
  (CameraFades|StartCameraFade :self _returnvalue :FromAlpha 1.0 :Duration _fade_time :bShouldFadeAudio true :bHoldWhenFinished true))

(event Custom|Doors_OpenClose
  ;[0 0 0] OPEN DOORS
  (if (not (Variables|Default|GetbIsPlay))
    (if (Variables|Default|Getdoor%20open)
      (CallFunction|DoorsClose)
      (else
        (CallFunction|DoorsOpen)))))

(event Custom|Fade_OUT
  (bind _returnvalue (Game|GetPlayerCameraManager 0))
  (bind _fade_time (Variables|Default|GetFade%20time))
  ;[0 0 0] FADE
  (Class|PlayerCameraManager|SetManualCameraFade :self _returnvalue :bInFadeAudio true)
  (Utilities|FlowControl|Delay _fade_time)
  (CameraFades|StartCameraFade :self _returnvalue :ToAlpha 1.0 :Duration _fade_time :bShouldFadeAudio true :bHoldWhenFinished true))

(event Custom|Doors_Close
  ;[0 0 0] OPEN DOORS
  (if (Variables|Default|Getdoor%20open)
    (if (not (Variables|Default|GetbIsPlay))
      (Variables|Default|SetbIsPlay true)
      (bind _returnvalue (Actor|GetActorOfClass "/Script/LevelSequence.LevelSequenceActor"))
      (Class|MovieSceneSequencePlayer|PlayReverse (Variables|/Script/LevelSequence.LevelSequenceActor|GetSequencePlayer _returnvalue))
      (Utilities|FlowControl|Delay 1.0)
      (Default|UpdateWidgetDoor (Variables|Default|GetW_Menu))
      (Variables|Default|SetbIsPlay false)
      (Variables|Default|Setdoor%20open false)
      (CallFunction|SimpleCaptureViews))))

(event Custom|Doors_Open
  ;[0 0 0] OPEN DOORS
  (if (not (Variables|Default|Getdoor%20open))
    (if (not (Variables|Default|GetbIsPlay))
      (Variables|Default|SetbIsPlay true)
      (bind _returnvalue (Actor|GetActorOfClass "/Script/LevelSequence.LevelSequenceActor"))
      (Sequencer|Player|Play (Variables|/Script/LevelSequence.LevelSequenceActor|GetSequencePlayer _returnvalue) :!class /Script/MovieScene.MovieSceneSequencePlayer)
      (Utilities|FlowControl|Delay 1.0)
      (Default|UpdateWidgetDoor (Variables|Default|GetW_Menu) 1)
      (Variables|Default|SetbIsPlay false)
      (Variables|Default|Setdoor%20open true)
      (CallFunction|SimpleCaptureViews))))

(event Custom|Rot0Force
  (bind _world (Variables|Default|GetWorld))
  (bind _rotator (Variables|Default|GetROTATOR))
  (bind _returnvalue (Transformation|GetActorRotation _rotator))
  (bind _returnvalue_2 (Transformation|GetActorRotation _world))
  ;[0 0 0] ROT 0 FORCE
  (Utilities|IsValid _rotator
    (:Is%20Valid
      (Transformation|SetActorRotation _rotator (Math|Rotator|MakeRotator (.roll _returnvalue) (.pitch _returnvalue) 0.0)))
    (:Is%20Not%20Valid
      _))
  (Utilities|IsValid _world
    (:Is%20Valid
      (Transformation|SetActorRotation _world (Math|Rotator|MakeRotator (.roll _returnvalue_2) (.pitch _returnvalue_2) 0.0))
      (Default|UpdateSliderW (Variables|Default|GetW_Menu) 0.0))))

(event EventBeginPlay
  (Utilities|FlowControl|Sequence
    (:then_0
      (bind _asbp_pawn (Utilities|Casting|CastToBp_Pawn (Game|Player|GetPlayerPawn 0)))
      (Variables|Default|SetAs%20Bp%20Pawn _asbp_pawn))
    (:then_1
      (for _array_element (Variables|Default|GetConsole%20Commands)
        (Development|ExecuteConsoleCommand _array_element 0)))
    (:then_2
      (Input|SetInputModeGameandUI self 0 "DoNotLock" true false)
      (Utilities|FlowControl|Delay 4.0)
      (Variables|Default|SetbShowMouseCursor true))
    (:then_3)
    (:then_4
      (CallFunction|FadeStart)
      (CallFunction|CreateWidgets)
      (CallFunction|SimpleCaptureViews))
    (:then_5
      ;[0 0 0] Bind On All Connections Closed event (could use this event to do something when all stream connections are lost)
      (bind _returnvalue (Class|PixelStreamingBlueprints|GetPixelStreamingDelegates))
      (EventDispatchers|BindEventtoOnAllConnectionsClosed _returnvalue (delegate Custom|Reset_Level_When_Connections_Closed_Event))
      ;[0 0 0] Bind On New Connection started event (could use this event to do something when a new stream connections is started)
      (EventDispatchers|BindEventtoOnNewConnection _returnvalue (delegate Custom|New_Connection_Started))
      ;[0 0 0] Get pixel streaming input and fire an event when new input is received
      (EventDispatchers|BindEventtoOnInputEvent (Variables|Default|GetPixelStreamingInput) (delegate Custom|Input_Recieved_Event)))))

(event Input|MouseEvents|MouseX
  (params (AxisValue :type Float%20%28single-precision%29))
  ;[0 0 0] MOUSE
  (if (Variables|Default|Getpressed)
    (Variables|Default|SetAxis%20Value AxisValue)
    (Class|Actor|AddActorWorldRotation (Variables|Default|GetROTATOR) (Math|Rotator|MakeRotator 0.0 0.0 (* (* (Variables|Default|GetAxis%20Value) -1.0) 6.0)))))

(event Input|KeyboardEvents|R
  (params (Key :type Key%20Structure :default "None"))
  ;[0 0 0] RESTART LEVEL
  (:Pressed
    (bind _returnvalue (Game|GetCurrentLevelName true))
    (Game|OpenLevel(byName) (Utilities|String|StringToName _returnvalue))))

(event Input|MouseEvents|LeftMouseButton
  (params (Key :type Key%20Structure :default "None"))
  ;[0 0 0] MOUSE
  (:Pressed
    (Variables|Default|Setpressed true))
  (:Released
    (Default|UpdateSliderW (Variables|Default|GetW_Menu) (.yaw (Transformation|GetActorRotation (Variables|Default|GetROTATOR))))
    (Variables|Default|Setpressed false)))

(event Input|MouseEvents|RightMouseButton
  (params (Key :type Key%20Structure :default "None"))
  ;[0 0 0] MOUSE
  (:Pressed
    (Variables|Default|Setpressed true))
  (:Released
    (Default|UpdateSliderW (Variables|Default|GetW_Menu) (.yaw (Transformation|GetActorRotation (Variables|Default|GetROTATOR))))
    (Variables|Default|Setpressed false)))

(event Input|MouseEvents|MouseWheelUp
  (params (Key :type Key%20Structure :default "None"))
  (bind _world (Variables|Default|GetWorld))
  (bind _rotator (Variables|Default|GetROTATOR))
  (bind _returnvalue (Transformation|GetActorRotation _world))
  (bind _returnvalue_2 (Transformation|GetActorRotation _rotator))
  (bind _returnvalue_3 (+ (.yaw _returnvalue) 1e+01))
  ;[0 0 0] ROTATOR - WHEEL
  (:Pressed
    (if (Variables|Default|GetbCanWheel)
      (Transformation|SetActorRotation _rotator (Math|Rotator|MakeRotator (.roll _returnvalue_2) (.pitch _returnvalue_2) (+ (.yaw _returnvalue_2) 1e+01)))
      (Transformation|SetActorRotation _world (Math|Rotator|MakeRotator (.roll _returnvalue) (.pitch _returnvalue) _returnvalue_3))
      (CallFunction|SimpleCaptureViews)
      (Default|UpdateSliderW (Variables|Default|GetW_Menu) _returnvalue_3))))

(event Input|MouseEvents|MouseWheelDown
  (params (Key :type Key%20Structure :default "None"))
  (bind _rotator (Variables|Default|GetROTATOR))
  (bind _world (Variables|Default|GetWorld))
  (bind _returnvalue (Transformation|GetActorRotation _rotator))
  (bind _returnvalue_2 (Transformation|GetActorRotation _world))
  (bind _returnvalue_3 (- (.yaw _returnvalue_2) 1e+01))
  ;[0 0 0] ROTATOR - WHEEL
  (:Pressed
    (if (Variables|Default|GetbCanWheel)
      (Transformation|SetActorRotation _rotator (Math|Rotator|MakeRotator (.roll _returnvalue) (.pitch _returnvalue) (- (.yaw _returnvalue) 1e+01)))
      (Transformation|SetActorRotation _world (Math|Rotator|MakeRotator (.roll _returnvalue_2) (.pitch _returnvalue_2) _returnvalue_3))
      (CallFunction|SimpleCaptureViews)
      (Default|UpdateSliderW (Variables|Default|GetW_Menu) _returnvalue_3))))

(event Input|TouchEvents|InputTouch
  (params (Location :type Vector) (FingerIndex :type ETouchIndex%20Enum)))

(fn ConstructionScript)

(fn GetMaterialName
  (params (Thumbnail :type Object%20Object%20Reference) (Material :type Object%20Object%20Reference))
  (return (Utilities|String|Contains (Utilities|String|Replace (Utilities|GetObjectName Thumbnail) "T_") (Utilities|String|Replace (Utilities|GetObjectName Material) "MI_"))))
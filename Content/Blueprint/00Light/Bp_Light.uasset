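; Configurable light actor that becomes a point, rect or spot light, or a disc lamp with a rect light sized to match.
; The construction script destroys the unselected light components, applies intensity and runs the setup function that pushes exposed properties to the remaining light.
; With ShowDisc on, it adds a scaled disc mesh at construction.
; TurnLight toggles intensity between zero and the set value, swapping the disc material between invisible and lit.
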(fn ConstructionScript
  (bind _rectlight (Variables|Components|GetRectLight))
  (bind _rectlight_2 (Variables|Components|GetRectLight))
  (bind _spotlight (Variables|Components|GetSpotLight))
  (bind _pointlight (Variables|Components|GetPointLight))
  (Utilities|FlowControl|Sequence
    (:then_0
      ;[0 0 0] SELECT lIGHT
      (if (Variables|0-Disc|GetShowDisc)
        (Components|DestroyComponent (Variables|Components|GetSpotLight))
        (CallFunction|DiscCreate)
        (else
          (CallFunction|DiscDelete)
          (switch Utilities|FlowControl|Switch|SwitchonStruct_LightSelector (Variables|0-Settings|GetSelector)
            (:NewEnumerator0
              (Components|DestroyComponent _rectlight_2))
            (:NewEnumerator1
              (Components|DestroyComponent (Variables|Components|GetSpotLight)))
            (:NewEnumerator2
              (Components|DestroyComponent _rectlight_2))))))
    (:then_1
      ;[0 0 0] INTENSITY & UNITS
      (Utilities|IsValid _spotlight
        (:Is%20Valid
          (Rendering|Components|Light|SetIntensity _spotlight (Variables|0-Settings|GetIntensity)))
        (:Is%20Not%20Valid
          _))
      (Utilities|IsValid _rectlight
        (:Is%20Valid
          (Rendering|Components|Light|SetIntensity _rectlight (Variables|0-Settings|GetIntensity)))
        (:Is%20Not%20Valid
          _))
      (Utilities|IsValid _pointlight
        (:Is%20Valid
          (Rendering|Components|Light|SetIntensity _pointlight (Variables|0-Settings|GetIntensity)))))
    (:then_2
      (if (Variables|0-Disc|GetShowDisc)
        ;[0 0 0] LIGHT SETUP
        (Utilities|IsValid (Variables|Components|GetRectLight) :!label _label
          (:Is%20Valid
            (CallFunction|SetupRectlight)))
        (else
          (switch Utilities|FlowControl|Switch|SwitchonStruct_LightSelector (Variables|0-Settings|GetSelector)
            (:NewEnumerator0
              (Utilities|IsValid (Variables|Components|GetPointLight)
                (:Is%20Valid
                  (CallFunction|SetupPointlight))))
            (:NewEnumerator1
              (goto _label))
            (:NewEnumerator2
              (Utilities|IsValid (Variables|Components|GetSpotLight)
                (:Is%20Valid
                  (CallFunction|SetupSpotlight))))))))))

(fn TurnLight
  (bind _rectlight (Variables|Components|GetRectLight))
  (bind _disc (Variables|Default|GetDisc))
  (bind _pointlight (Variables|Components|GetPointLight))
  (bind _intensity (Variables|0-Settings|GetIntensity))
  (bind _rectlight_2 (Variables|Components|GetRectLight))
  (bind _pointlight_2 (Variables|Components|GetPointLight))
  (bind _spotlight (Variables|Components|GetSpotLight))
  (bind _spotlight_2 (Variables|Components|GetSpotLight))
  (bind _disc_2 (Variables|Default|GetDisc))
  (if (Variables|Default|GetbOnLight)
    (Utilities|IsValid _disc_2
      (:Is%20Valid
        (Rendering|Material|SetMaterial _disc_2 0 "/Game/Materials/Master/M_Invisible01.M_Invisible01"))
      (:Is%20Not%20Valid
        _))
    (Utilities|IsValid _spotlight
      (:Is%20Valid
        (Rendering|Components|Light|SetIntensity _spotlight 0.0))
      (:Is%20Not%20Valid
        _))
    (Utilities|IsValid _rectlight_2
      (:Is%20Valid
        (Rendering|Components|Light|SetIntensity _rectlight_2 0.0))
      (:Is%20Not%20Valid
        _))
    (Utilities|IsValid _pointlight_2
      (:Is%20Valid
        (Rendering|Components|Light|SetIntensity _pointlight_2 0.0))
      (:Is%20Not%20Valid
        _))
    (Variables|Default|SetbOnLight false)
    (else
      (Utilities|IsValid _disc
        (:Is%20Valid
          (Rendering|Material|SetMaterial _disc 0 "/Game/AutomotiveMaterials/Materials/Exterior/Lights/MI_Lamp_White.MI_Lamp_White"))
        (:Is%20Not%20Valid
          _))
      (Utilities|IsValid _spotlight_2
        (:Is%20Valid
          (Rendering|Components|Light|SetIntensity _spotlight_2 _intensity))
        (:Is%20Not%20Valid
          _))
      (Utilities|IsValid _rectlight
        (:Is%20Valid
          (Rendering|Components|Light|SetIntensity _rectlight _intensity))
        (:Is%20Not%20Valid
          _))
      (Utilities|IsValid _pointlight
        (:Is%20Valid
          (Rendering|Components|Light|SetIntensity _pointlight _intensity))
        (:Is%20Not%20Valid
          _))
      (Variables|Default|SetbOnLight true))))

(fn DiscCreate
  (bind _disc_size (Variables|0-Disc|GetDisc%20size))
  (bind _returnvalue (AddComponent|AddStaticMeshComponent false))
  (bind _output_get (Variables|Default|SetDisc _returnvalue))
  (Components|StaticMesh|SetStaticMesh _output_get "/Game/SM_DiscLight.SM_DiscLight")
  (Transformation|AttachComponentToComponent (Variables|Components|GetDefaultSceneRoot) 0 "None" "KeepRelative" "KeepRelative" "KeepRelative" true)
  (Transformation|SetRelativeTransform _output_get (Math|Transform|MakeTransform "0, 0, 0" "180.000000,0.000000,0.000000" (Math|Vector|MakeVector _disc_size _disc_size _disc_size)) false false)
  (return))

(fn DiscDelete
  (bind _disc (Variables|Default|GetDisc))
  (if (Utilities|IsValid _disc)
    (Components|DestroyComponent _disc))
  (return))

(fn SetupRectlight
  (bind _disc_size (Variables|0-Disc|GetDisc%20size))
  (bind _rectlight (Variables|Components|GetRectLight))
  (bind _returnvalue (* _disc_size 2e+02))
  ;[0 0 0] REC LIGHT
  (Rendering|Lighting|SetAttenuationRadius _rectlight (Variables|0-Settings|GetAttenuation%20Radius))
  (Rendering|Components|Light|SetLightColor _rectlight (Variables|0-Settings|GetColor) true)
  (if (Variables|0-Disc|GetShowDisc)
    (Class|RectLightComponent|SetSourceWidth _rectlight _returnvalue)
    (Class|RectLightComponent|SetSourceHeight _rectlight _returnvalue)
    (else
      (Class|RectLightComponent|SetSourceWidth _rectlight (Variables|0-RectLight|GetWidth))
      (Class|RectLightComponent|SetSourceHeight _rectlight (Variables|0-RectLight|GetHeight))))
  (Class|RectLightComponent|SetBarnDoorAngle _rectlight (Variables|0-RectLight|GetBarn%20Door%20Angle))
  (Class|RectLightComponent|SetBarnDoorLength _rectlight (Variables|0-RectLight|GetBarn%20Door%20Length))
  (Class|LightComponent|SetUseTemperature _rectlight (Variables|0-Settings|GetUse%20Temperature))
  (Class|LightComponent|SetTemperature _rectlight (Variables|0-Settings|GetTemperature))
  (Class|LightComponent|SetVolumetricScatteringIntensity _rectlight (Variables|0-Settings|GetVolumetric%20Scattering%20intensity))
  (Class|LightComponent|SetIndirectLightingIntensity _rectlight (Variables|0-Settings|GetIndirect%20Lighting%20Intensity))
  (return))

(fn SetupPointlight
  (bind _pointlight (Variables|Components|GetPointLight))
  ;[0 0 0] POINT LIGHT
  (Rendering|Lighting|SetAttenuationRadius _pointlight (Variables|0-Settings|GetAttenuation%20Radius))
  (Rendering|Components|Light|SetLightColor _pointlight (Variables|0-Settings|GetColor) true)
  (Class|PointLightComponent|SetSourceRadius _pointlight (Variables|0-PointLight|GetSource%20Radius))
  (Class|PointLightComponent|SetSourceLength _pointlight (Variables|0-Settings|GetSource%20Length))
  (Class|LightComponent|SetUseTemperature _pointlight (Variables|0-Settings|GetUse%20Temperature))
  (Class|LightComponent|SetTemperature _pointlight (Variables|0-Settings|GetTemperature))
  (Class|LightComponent|SetVolumetricScatteringIntensity _pointlight (Variables|0-Settings|GetVolumetric%20Scattering%20intensity))
  (Class|LightComponent|SetIndirectLightingIntensity _pointlight (Variables|0-Settings|GetIndirect%20Lighting%20Intensity))
  (return))

(fn SetupSpotlight
  (bind _spotlight (Variables|Components|GetSpotLight))
  ;[0 0 0] SPOT LIGHT
  (Rendering|Lighting|SetAttenuationRadius _spotlight (Variables|0-Settings|GetAttenuation%20Radius))
  (Rendering|Components|Light|SetLightColor _spotlight (Variables|0-Settings|GetColor) true)
  (Class|PointLightComponent|SetSourceRadius _spotlight (Variables|0-PointLight|GetSource%20Radius))
  (Class|PointLightComponent|SetSourceLength _spotlight (Variables|0-Settings|GetSource%20Length))
  (Class|PointLightComponent|SetSoftSourceRadius _spotlight (Variables|0-SpotLight|GetSoft%20Source%20Radius))
  (Rendering|Lighting|SetInnerConeAngle _spotlight (Variables|0-SpotLight|GetInner%20Cone%20Angle))
  (Rendering|Lighting|SetOuterConeAngle _spotlight (Variables|0-SpotLight|GetOuter%20Cone%20Angle))
  (Class|LightComponent|SetUseTemperature _spotlight (Variables|0-Settings|GetUse%20Temperature))
  (Class|LightComponent|SetTemperature _spotlight (Variables|0-Settings|GetTemperature))
  (Class|LightComponent|SetVolumetricScatteringIntensity _spotlight (Variables|0-Settings|GetVolumetric%20Scattering%20intensity))
  (Class|LightComponent|SetIndirectLightingIntensity _spotlight (Variables|0-Settings|GetIndirect%20Lighting%20Intensity)))
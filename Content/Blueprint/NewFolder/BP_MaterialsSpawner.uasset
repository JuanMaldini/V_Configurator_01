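; BP_MaterialsSpawner builds lookup maps that pair switchable material instances with thumbnail textures, split into metal, textile, exterior wood and interior wood.
; ReCollect clears these lists, then scans the thumbnail folder and each category's material folder through the Asset Registry.
; Pairing is by name: a thumbnail matches when its name without "T_" contains the material's name without "MI_", and the last match wins.
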(fn ConstructionScript)

(fn Re-Collect
  (bind _returnvalue (Class|AssetRegistryHelpers|GetAssetRegistry))
  ;[0 0 0 0.5] COLLECT MATERIAL INSTANCES
  (Utilities|FlowControl|Sequence
    (:then_0
      (CallFunction|Clear)
      (Utilities|FlowControl|Sequence
        (:then_0
          (bind _outassetdata (Class|AssetRegistry|GetAssetsbyPath _returnvalue "/Game/Thumbnails/" true false))
          (for _array_element _outassetdata
            (bind _astexture (Utilities|Casting|CastToTexture (Class|AssetRegistryHelpers|GetAsset _array_element)))
            (Utilities|Array|AddUnique (Variables|Default|GetThumbnails) _astexture)))
        (:then_1
          (bind _outassetdata_2 (Class|AssetRegistry|GetAssetsbyPath _returnvalue "/Game/Materials/Instances/SwitchMaterials/METAL/" true false))
          (for _array_element_2 _outassetdata_2
            (bind _asmaterial_instance (Utilities|Casting|CastToMaterialInstance (Class|AssetRegistryHelpers|GetAsset _array_element_2)))
            (for _array_element_3 (Variables|Default|GetThumbnails)
              (if (CallFunction|GetMaterialName _array_element_3 _asmaterial_instance)
                (Utilities|Map|Add (Variables|Default|GetMaterialList_Metal) _asmaterial_instance _array_element_3)))))
        (:then_2
          (bind _outassetdata_3 (Class|AssetRegistry|GetAssetsbyPath _returnvalue "/Game/Materials/Instances/SwitchMaterials/TEXTILE/" true false))
          (for _array_element_4 _outassetdata_3
            (bind _asmaterial_instance_2 (Utilities|Casting|CastToMaterialInstance (Class|AssetRegistryHelpers|GetAsset _array_element_4)))
            (for _array_element_5 (Variables|Default|GetThumbnails)
              (if (CallFunction|GetMaterialName _array_element_5 _asmaterial_instance_2)
                (Utilities|Map|Add (Variables|Default|GetMaterialList_Textile) _asmaterial_instance_2 _array_element_5)))))
        (:then_3
          (bind _outassetdata_4 (Class|AssetRegistry|GetAssetsbyPath _returnvalue "/Game/Materials/Instances/SwitchMaterials/WOOD_EXTERIOR/" true false))
          (for _array_element_6 _outassetdata_4
            (bind _asmaterial_instance_3 (Utilities|Casting|CastToMaterialInstance (Class|AssetRegistryHelpers|GetAsset _array_element_6)))
            (for _array_element_7 (Variables|Default|GetThumbnails)
              (if (CallFunction|GetMaterialName _array_element_7 _asmaterial_instance_3)
                (Utilities|Map|Add (Variables|Default|GetMaterialList_WoodExt) _asmaterial_instance_3 _array_element_7)))))
        (:then_4
          (bind _outassetdata_5 (Class|AssetRegistry|GetAssetsbyPath _returnvalue "/Game/Materials/Instances/SwitchMaterials/WOOD_INTERIOR/" true false))
          (for _array_element_8 _outassetdata_5
            (bind _asmaterial_instance_4 (Utilities|Casting|CastToMaterialInstance (Class|AssetRegistryHelpers|GetAsset _array_element_8)))
            (for _array_element_9 (Variables|Default|GetThumbnails)
              (if (CallFunction|GetMaterialName _array_element_9 _asmaterial_instance_4)
                (Utilities|Map|Add (Variables|Default|GetMaterialList_WoodInt) _asmaterial_instance_4 _array_element_9)))))))
    (:then_1
      (return))))

(fn Clear
  (Utilities|Array|Clear (Variables|Default|GetThumbnails))
  (Utilities|Map|Clear (Variables|Default|GetMaterialList_Metal))
  (Utilities|Map|Clear (Variables|Default|GetMaterialList_Textile))
  (Utilities|Map|Clear (Variables|Default|GetMaterialList_WoodInt))
  (Utilities|Map|Clear (Variables|Default|GetMaterialList_WoodExt)))

(fn GetMaterialName
  (params (Thumbnail :type Object%20Object%20Reference) (Material :type Object%20Object%20Reference))
  (return (Utilities|String|Contains (Utilities|String|Replace (Utilities|GetObjectName Thumbnail) "T_") (Utilities|String|Replace (Utilities|GetObjectName Material) "MI_"))))
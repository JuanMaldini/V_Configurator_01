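; Material switcher actor that swaps metal, textile and exterior or interior wood materials on tagged static mesh actors.
; It caches all StaticMeshActors after BeginPlay, then matches SWITCH tags by category and parses the material slot index from the tag text.
; SwitchMaterial applies a given material, while SwitchRandom draws from BP_MaterialsSpawner lists but returns after the first category.
; Both then call SimpleCaptureViews on Bp_Controller.
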(event EventBeginPlay
  (Utilities|FlowControl|Sequence
    (:then_0
      (Utilities|FlowControl|Delay 0.4)
      (CallFunction|CollectActors))
    (:then_1
      (bind _asbp_controller (Utilities|Casting|CastToBp_Controller (Game|GetPlayerController 0)))
      (Variables|Default|SetAs%20Bp%20Controller _asbp_controller))))

(fn ConstructionScript)

(fn SwitchMaterial
  (params (Material :type Material%20Interface%20Object%20Reference) (Material%20Place :type Enum_Material%20Enum :default "NewEnumerator2"))
  (Variables|Default|Setmat_to_set Material)
  (for _array_element (Variables|Default|GetsceneActors)
    (for _array_element_2 (Variables|/Script/Engine.Actor|GetTags _array_element)
      (if (Utilities|String|Contains (Utilities|String|ToString(Name) _array_element_2) "SWITCH")
        (Variables|Default|SetCurrent%20Str (Utilities|String|ToString(Name) _array_element_2))
        (Variables|Default|SetCurrectActorLoop _array_element)
        (switch Utilities|FlowControl|Switch|SwitchonEnum_Material Material%20Place
          (:NewEnumerator2
            (if (CallFunction|ContainsS "METAL")
              (Utilities|FindIndexforMaterial)))
          (:NewEnumerator3
            (if (CallFunction|ContainsS "TEXTILE")
              (Utilities|FindIndexforMaterial)))
          (:NewEnumerator0
            (if (CallFunction|ContainsS "WOOD EXTERIOR")
              (Utilities|FindIndexforMaterial)))
          (:NewEnumerator1
            (if (CallFunction|ContainsS "WOOD INTERIOR")
              (Utilities|FindIndexforMaterial)))))))
  (bind _asbp_controller (Utilities|Casting|CastToBp_Controller (Game|GetPlayerController 0)))
  (Default|SimpleCaptureViews _asbp_controller)
  (return))

(fn CollectActors
  (bind _outactors (Actor|GetAllActorsOfClass "/Script/Engine.StaticMeshActor"))
  (Variables|Default|SetsceneActors _outactors)
  (return))

(fn ContainsS
  (params (In :type String))
  (return (Utilities|String|Contains (Variables|Default|GetCurrent%20Str) In)))

(fn ContainsI
  (params (In :type Integer))
  (return (Utilities|String|Contains (Variables|Default|GetCurrent%20Str) (Utilities|String|ToString(Integer) In))))

(fn SwitchRandom
  (bind _as_bp_controller (Variables|Default|GetAs%20Bp%20Controller))
  (for _array_element (Variables|Default|GetAllMaterialsStr)
    (bind _output_get (Variables|Default|Setcurrent_mat _array_element))
    (bind _returnvalue (Actor|GetActorOfClass "/Game/Blueprint/NewFolder/BP_MaterialsSpawner.BP_MaterialsSpawner_C"))
    (switch string _output_get
      (:METAL
        (bind _keys (Utilities|Map|Keys (Variables|/Game/Blueprint/NewFolder/BP_MaterialsSpawner.BP_MaterialsSpawner_C|GetMaterialList_Metal _returnvalue)))
        (Variables|Default|Setmat_to_set (.OutItem (Utilities|Array|Random _keys))))
      (:TEXTILE
        (bind _keys_2 (Utilities|Map|Keys (Variables|/Game/Blueprint/NewFolder/BP_MaterialsSpawner.BP_MaterialsSpawner_C|GetMaterialList_Textile _returnvalue)))
        (Variables|Default|Setmat_to_set (.OutItem (Utilities|Array|Random _keys_2))))
      (:WOOD%20EXTERIOR
        (bind _keys_3 (Utilities|Map|Keys (Variables|/Game/Blueprint/NewFolder/BP_MaterialsSpawner.BP_MaterialsSpawner_C|GetMaterialList_WoodExt _returnvalue)))
        (Variables|Default|Setmat_to_set (.OutItem (Utilities|Array|Random _keys_3))))
      (:WOOD%20INTERIOR
        (bind _keys_4 (Utilities|Map|Keys (Variables|/Game/Blueprint/NewFolder/BP_MaterialsSpawner.BP_MaterialsSpawner_C|GetMaterialList_WoodInt _returnvalue)))
        (Variables|Default|Setmat_to_set (.OutItem (Utilities|Array|Random _keys_4)))))
    (for _array_element_2 (Variables|Default|GetsceneActors)
      (for _array_element_3 (Variables|/Script/Engine.Actor|GetTags _array_element_2)
        (if (Utilities|String|Contains (Utilities|String|ToString(Name) _array_element_3) "SWITCH")
          (Variables|Default|SetCurrent%20Str (Utilities|String|ToString(Name) _array_element_3))
          (Variables|Default|SetCurrectActorLoop _array_element_2)
          (if (CallFunction|ContainsS (Variables|Default|Getcurrent_mat))
            (Utilities|FindIndexforMaterial)))))
    (bind _asbp_controller (Utilities|Casting|CastToBp_Controller (Game|GetPlayerController 0))
      (:then
        (Default|SimpleCaptureViews _asbp_controller))
      (:CastFailed
        _))
    (return))
  (Utilities|IsValid _as_bp_controller
    (:Is%20Valid
      (Default|SimpleCaptureViews _as_bp_controller))))
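; Camera pawn that glides between viewpoints marked by Bp_Target actors in the level.
; BlendCamera searches all targets for a match on either the Views enum or the LocationVar number, selected by the Enum flag.
; If that target is over 50 units away, a timeline lerps the pawn's transform, with sweep, to the target's Arrow transform.
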(event Custom|Blend%20Camera
  (params (Camera%20Location%20Number :type Integer) (Camera%20Location%20Enum :type Enum_Views%20Enum :default "NewEnumerator0") (Enum? :type Boolean))
  (bind _outactors (Actor|GetAllActorsOfClass "/Game/Blueprint/Bp_Target.Bp_Target_C"))
  (for _array_element _outactors
    (if Enum?
      (if (Utilities|Enum|Equal(Enum) (Variables|/Game/Blueprint/Bp_Target.Bp_Target_C|Getviews _array_element) Camera%20Location%20Enum)
        (if (> (Math|Vector|Distance(Vector) (Transformation|GetActorLocation _array_element) (Transformation|GetActorLocation self)) 5e+01) :!label _label
          (Variables|Default|SetDestination (Transformation|GetWorldTransform (Variables|/Game/Blueprint/Bp_Target.Bp_Target_C|GetArrow _array_element)))
          (Variables|Default|SetCurrent (Transformation|GetActorTransform))
          (bind _newtrack_0 (Timeline|Timeline PlayFromStart)
            (:Update
              (Transformation|SetActorTransform (Math|Transform|Lerp(Transform) (Variables|Default|GetCurrent) (Variables|Default|GetDestination) _newtrack_0) true)))))
      (elif (== (Variables|/Game/Blueprint/Bp_Target.Bp_Target_C|GetLocation%20var _array_element) Camera%20Location%20Number)
        (goto _label)))))

(event EventBeginPlay)

(fn ConstructionScript)